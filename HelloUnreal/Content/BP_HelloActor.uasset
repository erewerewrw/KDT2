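; BP_HelloActor is an actor that slides its Sphere component back and forth along relative X, apparently as a Blueprint practice piece.
; Tick moves the sphere by Speed scaled by delta time, flipping IsMoveRight once it reaches 500 or returns to 0.
; BeginPlay prints the actor's name and a completion message around an empty loop.
; Disconnected nodes hold unused experiments with loops, math, location and rotation.
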(event EventBeginPlay
  (Development|PrintString (Utilities|GetDisplayName self) true true "(R=0.615187,G=0.000000,B=1.000000,A=1.000000)" 6e+01)
  (Variables|Default|SetX축의%20값 (+ 1.0 1.0))
  (for _index (range 0 5)
    _)
  (Development|PrintString "complete" true true "(R=0.000000,G=0.660000,B=1.000000,A=1.000000)" 6e+01))

(event EventTick
  (params (DeltaSeconds :type Float%20%28single-precision%29))
  (bind _sphere (Variables|Default|GetSphere))
  (bind _sphere_2 (Variables|Default|GetSphere))
  (if (Variables|Default|GetisMoveRight)
    (Transformation|AddRelativeLocation _sphere_2 (Math|Vector|MakeVector (* (* DeltaSeconds 1.0) (Variables|Default|GetSpeed)) 0.0 0.0) false false)
    (if (>= (.x (Variables|/Script/Engine.SceneComponent|GetRelativeLocation _sphere_2)) 5e+02)
      (Variables|Default|SetisMoveRight false))
    (else
      (Transformation|AddRelativeLocation _sphere (Math|Vector|MakeVector (* (* DeltaSeconds -1.0) (Variables|Default|GetSpeed)) 0.0 0.0) false false)
      (if (<= (.x (Variables|/Script/Engine.SceneComponent|GetRelativeLocation _sphere)) 0.0)
        (Variables|Default|SetisMoveRight true)))))

(fn ConstructionScript)